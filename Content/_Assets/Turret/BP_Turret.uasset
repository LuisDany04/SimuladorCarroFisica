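; BP_Turret is an automated turret that tracks and shoots the nearest visible vehicle within its sensing range.
; Each tick it picks a target by sphere overlap and line-of-sight check, then turns its top mesh at constant speed with clamped pitch.
; When the cooldown has passed and a dot product confirms aim, it fires a burst of BP_Bullet actors, alternating left and right barrel sockets through a delayed DoN loop.
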(event Custom|Fire
  (Variables|Private|SetTimeOfLastFire (Utilities|Time|GetGameTimeinSeconds))
  (Utilities|FlowControl|Sequence
    (:then_0
      (goto _label Reset))
    (:then_1
      (Utilities|FlowControl|DoN 2 :!label _label
        (:Exit
          (Game|SpawnActorfromClass "/Game/_Assets/Turret/BP_Bullet.BP_Bullet_C" (Transformation|GetSocketTransform (Variables|Default|GetStaticMeshBarrelL) "FireSocket" "RTS_World") "Undefined" 0 0)
          (Utilities|FlowControl|Delay 0.2)
          (Game|SpawnActorfromClass "/Game/_Assets/Turret/BP_Bullet.BP_Bullet_C" (Transformation|GetSocketTransform (Variables|Default|GetStaticMeshBarrelR) "FireSocket" "RTS_World") "Undefined" 0 0)
          (Utilities|FlowControl|Delay 0.2)
          (goto _label))))))

(event EventTick
  (params (DeltaSeconds :type Float%20%28single-precision%29))
  (Private|FindBestTarget)
  (Variables|Private|GetTarget
    (:then
      (Private|UpdateTurretRotation DeltaSeconds)
      (Private|UptadeFire))
    (:else)))

(fn ConstructionScript)

(fn FindBestTarget
  (LocalVariables|SetBestDistance (+ (Variables|Constants|GetSensingRange) 1.0))
  (bind _outactors (Collision|SphereOverlapActors (Transformation|GetActorLocation) (Variables|Constants|GetSensingRange) (Utilities|Array|MakeArray "ObjectTypeQuery5") "/Script/Engine.Actor"))
  (for _array_element _outactors
    (bind _output_get (LocalVariables|SetCurrentTarget _array_element))
    (bind _output_get_2 (LocalVariables|SetCurrentDistance (Transformation|GetDistanceTo _output_get self)))
    (if (or (< _output_get_2 (LocalVariables|GetBestDistance)) (not (Utilities|IsValid (LocalVariables|GetBestTarget))))
      (bind _result (CallFunction|HasLineOfSight (Transformation|GetWorldLocation (Variables|Default|GetStaticMeshTop)) (Transformation|GetActorLocation (LocalVariables|GetCurrentTarget)) (Utilities|Array|MakeArray self (LocalVariables|GetCurrentTarget))))
      (if _result
        (LocalVariables|SetBestTarget (LocalVariables|GetCurrentTarget))
        (LocalVariables|SetBestDistance (LocalVariables|GetCurrentDistance)))))
  (Variables|Private|SetTarget (LocalVariables|GetBestTarget)))

(fn UpdateTurretRotation
  (params (DeltaSeconds :type Float%20%28double-precision%29))
  (bind _output_get (LocalVariables|SetNewRotation (Class|KismetMathLibrary|RInterptoConstant (Transformation|GetWorldRotation (Variables|Default|GetStaticMeshTop)) (Math|Rotator|FindLookatRotation (Transformation|GetWorldLocation (Variables|Default|GetStaticMeshTop)) (Transformation|GetActorLocation (Variables|Private|GetTarget))) DeltaSeconds (Variables|Constants|GetRotationSpeed))))
  (Transformation|SetWorldRotation (Variables|Default|GetStaticMeshTop) (Math|Rotator|MakeRotator (.roll _output_get) (Math|Float|ClampAngle (.pitch _output_get) -45.0 75.0) (.yaw _output_get)) false false))

(fn UptadeFire
  (if (> (- (Utilities|Time|GetGameTimeinSeconds) (Variables|Private|GetTimeOfLastFire)) (Variables|Constants|GetRateOfFire)) ; Has rate of fire cooldown
    (if (> (Math|Vector|DotProduct (Math|Vector|GetUnitDirection(Vector) (Transformation|GetWorldLocation (Variables|Default|GetStaticMeshTop)) (Transformation|GetActorLocation (Variables|Private|GetTarget))) (Math|Vector|GetForwardVector (Variables|Default|GetStaticMeshTop))) 0.99) ; La torreta ve el objetivo
      (CallFunction|Fire))))